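; BP_ObjetQuiFlotte_4 is a floating-object actor that moves along its local axes whenever another actor overlaps it.
; Each overlap flips a pair of booleans tracking odd and even visits, then restarts the Chronologie timeline from the start in either branch.
; The timeline update adds its track value as an unswept local offset, so movement accumulates per update rather than interpolating between fixed positions.
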(event Collision|EventActorBeginOverlap
  (params (OtherActor :type Actor%20Object%20Reference))
  (if (Variables|Default|Getjoueur%20est%20allé%20pour%20la%20nb%20paire%20fois)
    (Variables|Default|Setjoueur%20est%20allé%20pour%20nb%20impaire%20de%20fois true)
    (Variables|Default|Setjoueur%20est%20allé%20pour%20la%20nb%20paire%20fois false)
    (bind _nouvelle_piste_1 (Timeline|Chronologie PlayFromStart)
      (:Update
        (Transformation|AddActorLocalOffset _nouvelle_piste_1 false false)))
    (else
      (Variables|Default|Setjoueur%20est%20allé%20pour%20nb%20impaire%20de%20fois false)
      (Variables|Default|Setjoueur%20est%20allé%20pour%20la%20nb%20paire%20fois true)
      (Timeline|Chronologie PlayFromStart))))

(event EventBeginPlay
  (Variables|Default|Setjoueur%20est%20allé%20pour%20nb%20impaire%20de%20fois false)
  (Variables|Default|Setjoueur%20est%20allé%20pour%20la%20nb%20paire%20fois true))

(fn ConstructionScript)